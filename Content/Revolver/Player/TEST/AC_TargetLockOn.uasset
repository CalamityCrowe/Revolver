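; Test actor component that gives the Revolver player character a camera lock-on to a target.
; StartLock-on runs a Targeting System preset, takes the first result as the target and adds a loose lock-on gameplay tag.
; A looping timer interpolates control rotation toward the target until it is invalid or out of range, then clears it without removing the tag.
; Debug boxes, a range sphere and printed distance visualise the process.
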(event `self.ReceiveBeginPlay`
  ; We want to grab the owning player and ASC to keep as a reference for later use
  (bind _asrevolver_player_character (cast `RevolverPlayerCharacter` (`self.GetOwner`)))
  (bind _output_get (set `self.PlayerRef` _asrevolver_player_character))
  (set `self.ASC` (`AbilitySystemBlueprintLibrary.GetAbilitySystemComponent` _output_get)))

(event `Start Lock-on`
  (`KismetSystemLibrary.K2_ClearAndInvalidateTimerHandle` (`self.Lock Timer Handle`))
  (bind (_asynctaskproxy _targetinghandle) (`AsyncAction_PerformTargeting.PerformTargetingRequest` (`self.PlayerRef`) (`self.Targeting Data`))
    (:`Targeted`
      (for (_array_element _array_index) (`TargetingSubsystem.GetTargetingResultsActors` (subsystem `TargetingSubsystem`) _targetinghandle)
        (`self.Draw Debug box` _array_element _array_index)
        (if (== _array_index 0)
          (set `self.CurrentTarget` _array_element)))
      (`self.CurrentTarget`
        (:`then`
          (bind _returnvalue (`KismetSystemLibrary.K2_SetTimerDelegate` (delegate `Adjust Camera`) 0.01 true))
          (set `self.Lock Timer Handle` _returnvalue)
          (`AbilitySystemBlueprintLibrary.AddLooseGameplayTags` (`self.PlayerRef`) (`self.Lock on tag`)))
        (:`else`)))))

(event `Adjust Camera`
  (bind _playerref (`self.PlayerRef`))
  (`Controller.SetControlRotation` (`Pawn.GetController` (`self.PlayerRef`)) (`KismetMathLibrary.RInterpTo` (`Pawn.GetControlRotation` _playerref) (`KismetMathLibrary.FindLookAtRotation` (`Actor.K2_GetActorLocation` _playerref) (`Actor.K2_GetActorLocation` (`self.CurrentTarget`))) (`GameplayStatics.GetWorldDeltaSeconds`) 5.0))
  (if (`self.Still in range of owner` 1000.0)
    (`self.Draw Debug Capsule` 1000.0 (`self.PlayerRef`))
    (else
      (`KismetSystemLibrary.K2_ClearAndInvalidateTimerHandle` (`self.Lock Timer Handle`))
      (set `self.CurrentTarget` null))))

(fn `Draw Debug box`
  (params (`Target Actor` :type "Actor Object Reference") (Index :type Integer))
  (locals (`Debug Colour` :type "LinearColor Structure"))
  (bind _target_actor (`local.Target Actor`))
  (`/Engine/EditorBlueprintResources/StandardMacros.IsValid` `Target Actor`
    (:`Is Valid`
      (switch `int` Index
        (:`Default`
          (set `local.Debug Colour` (struct :`R` 1.0 :`B` 0.121963 :`A` 1.0)))
        (:`0`
          (set `local.Debug Colour` (struct :`R` 0.012654 :`G` 1.0 :`A` 1.0)))
        (:`1`
          (set `local.Debug Colour` (struct :`R` 1.0 :`G` 0.874834 :`A` 1.0))))
      (`KismetSystemLibrary.DrawDebugBox` (`Actor.K2_GetActorLocation` _target_actor) (`.BoxExtent` (`Actor.GetActorBounds` _target_actor false false)) (`local.Debug Colour`) (struct) 3.0 2.0))))

(fn `Draw Debug Capsule`
  (params (Radius :type "Float (double-precision)") (actor :type "Actor Object Reference"))
  (`KismetSystemLibrary.DrawDebugSphere` (`Actor.K2_GetActorLocation` actor) Radius 32 (struct :`G` 0.778733 :`B` 1.0 :`A` 1.0) 0.1 2.0))

(fn `Still in range of owner`
  (params (`Max Distance` :type "Float (double-precision)"))
  (returns (`Still In Range` :type Boolean))
  (bind _returnvalue (`KismetMathLibrary.VSize` (- (`Actor.K2_GetActorLocation` (`self.PlayerRef`)) (`Actor.K2_GetActorLocation` (`self.CurrentTarget`)))))
  (if (and (`KismetSystemLibrary.IsValid` (`self.PlayerRef`)) (`KismetSystemLibrary.IsValid` (`self.CurrentTarget`)))
    (`KismetSystemLibrary.PrintText` (`|FormatText` "Duration: {Duration}" _returnvalue))
    (if (< _returnvalue (`local.Max Distance`))
      (return true)
      (else
        (return false)))
    (else
      (return false))))