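; GA_PassiveHealth is a toggle-style passive Gameplay Ability that periodically applies a health-related effect to its owner for a recurring cost.
; When the montage's trigger event arrives, it commits the ability, builds an effect spec with a SetByCaller magnitude and starts a looping timer.
; Each tick pays the cost and applies the spec, ending the ability once the cost becomes unaffordable.
; Ending removes the effect and clears the timer.
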(event `self.MontageStarted`
  (`AbilityTask_WaitGameplayEvent.WaitGameplayEvent` (`self.MontageTriggeredTag`) null
    (:`EventReceived`
      (`/Engine/EditorBlueprintResources/StandardMacros.IsValid` (`AbilitySystemBlueprintLibrary.GetAbilitySystemComponent` (`self.GetAvatarActorFromActorInfo`))
        (:`Is Valid`
          (bind _returnvalue (`self.K2_CheckAbilityCost`))
          (if _returnvalue
            (bind _returnvalue_2 (`self.K2_CommitAbility`))
            (if _returnvalue_2
              (bind _returnvalue_3 (`AbilitySystemBlueprintLibrary.AssignTagSetByCallerMagnitude` (`self.MakeOutgoingGameplayEffectSpec` (`self.EffectClass`)) (`self.EffectMagnitudeTag`) (`self.EffectMagnitude`)))
              (set `self.Effect Spec` _returnvalue_3)
              (bind _returnvalue_4 (`KismetSystemLibrary.K2_SetTimerDelegate` (`|CreateDelegate` :!event `Apply Passive Effect`) 2.0 true))
              (set `self.Effect Timer` _returnvalue_4)
              (else
                (`self.K2_EndAbility`)))))))))

(event `self.K2_OnEndAbility`
  (params (bWasCancelled :type Boolean))
  (`AbilitySystemComponent.RemoveActiveGameplayEffectBySourceEffect` (`AbilitySystemBlueprintLibrary.GetAbilitySystemComponent` (`self.GetAvatarActorFromActorInfo`)) (`self.EffectClass`) null -1)
  (`KismetSystemLibrary.K2_ClearAndInvalidateTimerHandle` (`self.Effect Timer`))
  (set `self.Effect Spec` (struct)))

(event `Apply Passive Effect`
  (bind _returnvalue (`self.K2_CommitAbilityCost` false))
  (if _returnvalue
    (`AbilitySystemComponent.BP_ApplyGameplayEffectSpecToSelf` (`AbilitySystemBlueprintLibrary.GetAbilitySystemComponent` (`self.GetAvatarActorFromActorInfo`)) (`self.Effect Spec`))
    (bind _returnvalue_2 (`self.K2_CheckAbilityCost`))
    (if (not _returnvalue_2)
      (`self.K2_EndAbility`))
    (else
      (`self.K2_EndAbility`))))