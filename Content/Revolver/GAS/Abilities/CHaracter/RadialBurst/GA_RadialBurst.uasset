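; GA_RadialBurst is the player's Radial Burst gameplay ability, and its Blueprint graph handles only the camera framing while the ability runs.
; On activation it pulls the RevolverPlayerCharacter's camera boom back and centers it higher above the character.
; On end it sets the boom to a closer over-the-shoulder offset using hardcoded values rather than cached ones, with both changes applied instantly without interpolation.
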(event `self.K2_ActivateAbility`
  (bind _cameraboom (`RevolverPlayerCharacter.CameraBoom` (cast `RevolverPlayerCharacter` (`self.GetAvatarActorFromActorInfo`) :!pure true)))
  (set `SpringArmComponent.SocketOffset` (0.0 0.0 100.0) _cameraboom)
  (set `SpringArmComponent.TargetArmLength` 600.0 _cameraboom))

(event `self.K2_OnEndAbility`
  (params (bWasCancelled :type Boolean))
  (bind _cameraboom (`RevolverPlayerCharacter.CameraBoom` (cast `RevolverPlayerCharacter` (`self.GetAvatarActorFromActorInfo`) :!pure true)))
  (set `SpringArmComponent.SocketOffset` (0.0 50.0 60.0) _cameraboom)
  (set `SpringArmComponent.TargetArmLength` 300.0 _cameraboom))